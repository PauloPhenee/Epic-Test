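; Player controller that drives a charge-and-fire ball weapon through a crosshair widget, apparently as a test.
; BeginPlay pushes the crosshair onto a widget stack and sets up Enhanced Input.
; Holding charge runs a timeline that fills empty BallCharge slots in sequence, animating the reticule.
; Releasing fire spends the highest charged slot, gated by ReadyToFire, and resets the fire-rate timer that Tick advances.
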(event `self.ReceiveBeginPlay`
  (bind _returnvalue (`|CreateWidget` "/Game/UI/WBP_WidgetStack.WBP_WidgetStack_C" self))
  (bind _output_get (set `self.WidgetStack` _returnvalue))
  (`UserWidget.AddToViewport` _output_get 0)
  (bind _widget (`/Game/UI/WBP_WidgetStack.PushWidget` _output_get "NewEnumerator0" "/Game/UI/UI_Widgets/WBP_CrossHair.WBP_CrossHair_C"))
  (bind _aswbp_cross_hair (cast `/Game/UI/UI_Widgets/WBP_CrossHair` _widget))
  (bind _output_get_2 (set `self.Widget` _aswbp_cross_hair))
  (set `/Game/UI/UI_Widgets/WBP_CrossHair.FireRateRotationSpeed` (`self.WeaponFireRate`) _output_get_2)
  (`TimelineComponent.SetPlayRate` (`self.Charger`) (/ 1.0 (`self.WeaponChargeRate`)))
  (`EnhancedInputSubsystemInterface.AddMappingContext` (pcsubsystem `EnhancedInputLocalPlayerSubsystem` self) "/Game/Input/IMC_GameInput.IMC_GameInput" 0 (struct))
  (`WidgetBlueprintLibrary.SetInputMode_GameOnly` self)
  (set `self.bShowMouseCursor` false))

(event `EnhancedInput|/Game/Input/Input_Actions/IA_Charge`
  (params (ActionValue :type Boolean) (ElapsedSeconds :type "Float (double-precision)") (TriggeredSeconds :type "Float (double-precision)") (InputAction :type "InputAction Object Reference" :default "/Game/Input/Input_Actions/IA_Charge.IA_Charge"))
  (bind _widget (`self.Widget`))
  (:`Started`
    (`self.ChargeBall`)
    (`/Game/UI/UI_Widgets/WBP_CrossHair.Expande Reticule Anim` _widget))
  (:`Canceled`
    (`self.Stop Charge Ball` :!label _label)
    (`/Game/UI/UI_Widgets/WBP_CrossHair.Retract Reticule Anim` _widget))
  (:`Completed`
    (goto _label)))

(event `EnhancedInput|/Game/Input/Input_Actions/IA_Fire`
  (params (ActionValue :type Boolean) (ElapsedSeconds :type "Float (double-precision)") (TriggeredSeconds :type "Float (double-precision)") (InputAction :type "InputAction Object Reference" :default "/Game/Input/Input_Actions/IA_Fire.IA_Fire"))
  (:`Completed`
    (bind _index (`self.Get Next Available Ball`))
    (if (and (>= _index 0) (`self.ReadyToFire`))
      (`/Game/UI/UI_Widgets/WBP_CrossHair.Fire` (`self.Widget`) _index)
      (`KismetArrayLibrary.Array_Set` (`self.BallCharge`) _index)
      (set `self.WeaponFireRateTimer` 0.0))))

(event `ChargeBall`
  (bind _chargingindex (`self.ChargingIndex`))
  ; Charging Controller
  (bind _index (`self.Get Next Empty Ball` :!label _label_2))
  (bind _output_get (set `self.ChargingIndex` _index))
  (if (>= _output_get 0)
    (set `self.IsCharging` true)
    (bind (_direction _charge) (`Timeline|Charger` :!via `PlayFromStart` :!label _label_3)
      (:`Update`
        (`/Game/UI/UI_Widgets/WBP_CrossHair.Charge` (`self.Widget`) _charge _chargingindex))
      (:`Finished`
        (`KismetArrayLibrary.Array_Set` (`self.BallCharge`) _chargingindex true)
        (`/Game/UI/UI_Widgets/WBP_CrossHair.Stop Charge` (`self.Widget`) _chargingindex)
        (goto _label_2)))))

(event `Stop Charge Ball`
  ; Charging Controller
  (if (`self.IsCharging`)
    (`/Game/UI/UI_Widgets/WBP_CrossHair.Stop Charge` (`self.Widget`) (`self.ChargingIndex`))
    (set `self.IsCharging` false)
    (goto _label_3 :!via `Stop`)))

(event `self.ReceiveTick`
  (params (DeltaSeconds :type "Float (single-precision)"))
  ; Charging Controller
  (if (> (`self.WeaponFireRate`) (`self.WeaponFireRateTimer`))
    (set `self.WeaponFireRateTimer` (+ (`self.WeaponFireRateTimer`) DeltaSeconds))))

(fn `Get Next Available Ball`
  (returns (Index :type Integer))
  (bind (_arrayindex _arrayelement) (`/Engine/EditorBlueprintResources/StandardMacros.ReverseForEachLoop` (`self.BallCharge`))
    (:`LoopBody`
      (if _arrayelement
        (return _arrayindex)))
    (:`Completed`
      (return -1))))

(fn `Get Next Empty Ball`
  (returns (Index :type Integer))
  (for (_array_element _array_index) (`self.BallCharge`)
    (if (not _array_element)
      (return _array_index)))
  (return -1))

(fn `UserConstructionScript`)